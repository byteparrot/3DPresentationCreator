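; Player pawn for a slide presentation that moves its camera between SlideBP actors placed in the level.
; Gathers slides on construction, then sorts them by index on BeginPlay.
; Mouse, keyboard or touch input steps through them with wraparound, and a settings toggle blocks navigation.
; A timeline moves the camera by lerp or spline (reversed going back) while cross-fading content, then fires slide triggers and starts any auto-continue timer.
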(event Custom|GotoNextSlide
  (if (not (Variables|/PresentationPlugin/presentationUI.presentationUI_C|GetshowSettings (Variables|Default|GetpresentationUI)))
    (Utilities|Time|ClearandInvalidateTimerbyHandle (Variables|Default|GetautoContinueHandle))
    (Utilities|IsValid (Variables|Default|GetoldSlide)
      (:Is%20Valid
        (Default|SetContentAlpha (Variables|Default|GetoldSlide) 0.0))
      (:Is%20Not%20Valid
        _))
    (Utilities|IsValid (Utilities|Array|Get(acopy) (Variables|Default|GetSlideArray) (Variables|Default|Getindex))
      (:Is%20Valid
        (Variables|Default|SetoldSlide (Utilities|Array|Get(acopy) (Variables|Default|GetSlideArray) (Variables|Default|Getindex))))
      (:Is%20Not%20Valid
        _))
    (Math|Integer|IncrementInt (Variables|Default|Getindex)
      (:%20%20
        (Variables|Default|SetforwardDirection true)
        (if (>= (Variables|Default|Getindex) (Utilities|Array|Length (Variables|Default|GetSlideArray)))
          (Variables|Default|Setindex 0))
        (Variables|Default|Setoldtransform (Transformation|GetWorldTransform (Variables|Default|GetCamera)))
        (Utilities|ContinueifSlidesExist)
        (Utilities|IsValid (Utilities|Array|Get(acopy) (Variables|Default|GetSlideArray) (Variables|Default|Getindex))
          (:Is%20Valid
            (Variables|Default|Setnewtransform (Transformation|GetWorldTransform (Variables|/PresentationPlugin/SlideBP.SlideBP_C|GetArrow (Utilities|Array|Get(acopy) (Variables|Default|GetSlideArray) (Variables|Default|Getindex)))))
            (Components|Timeline|SetPlayRate (Variables|Default|GetTransition) (/ 1.0 (Variables|/PresentationPlugin/SlideBP.SlideBP_C|GettransitionDuration (select (Variables|Default|GetforwardDirection) (Utilities|Array|Get(acopy) (Variables|Default|GetSlideArray) (Variables|Default|Getindex)) (Variables|Default|GetoldSlide)))))
            (bind (_direction _smoothcurve _linearcurve) (Timeline|Transition PlayFromStart)
              (:Update
                (Transformation|SetWorldLocationAndRotation (Variables|Default|GetCamera) (Math|Vector|SelectVector (Spline|GetLocationatDistanceAlongSpline (Variables|/PresentationPlugin/SlideBP.SlideBP_C|GetSpline (select (Variables|Default|GetforwardDirection) (Utilities|Array|Get(acopy) (Variables|Default|GetSlideArray) (Variables|Default|Getindex)) (Variables|Default|GetoldSlide))) (* (select (Variables|Default|GetforwardDirection) _smoothcurve (- 1.0 _smoothcurve)) (Spline|GetSplineLength (Variables|/PresentationPlugin/SlideBP.SlideBP_C|GetSpline (select (Variables|Default|GetforwardDirection) (Utilities|Array|Get(acopy) (Variables|Default|GetSlideArray) (Variables|Default|Getindex)) (Variables|Default|GetoldSlide))))) "World") (Math|Vector|Lerp(Vector) (.location (Variables|Default|Getoldtransform)) (.location (Variables|Default|Getnewtransform)) _smoothcurve) (and (Variables|/PresentationPlugin/SlideBP.SlideBP_C|GethasTransitionBeginning (select (Variables|Default|GetforwardDirection) (Utilities|Array|Get(acopy) (Variables|Default|GetSlideArray) (Variables|Default|Getindex)) (Variables|Default|GetoldSlide))) (Variables|/PresentationPlugin/SlideBP.SlideBP_C|GetuseComplexPath (select (Variables|Default|GetforwardDirection) (Utilities|Array|Get(acopy) (Variables|Default|GetSlideArray) (Variables|Default|Getindex)) (Variables|Default|GetoldSlide))))) (Math|Rotator|Lerp(Rotator) (.rotation (Variables|Default|Getoldtransform)) (.rotation (Variables|Default|Getnewtransform)) _smoothcurve true) false false)
                (Utilities|IsValid (Variables|Default|GetoldSlide)
                  (:Is%20Valid
                    (Default|SetContentAlpha (Variables|Default|GetoldSlide) (- 1.0 _linearcurve)))
                  (:Is%20Not%20Valid
                    (Development|PrintString "A Slide is missing!" true true "(R=0.000000,G=0.660000,B=1.000000,A=1.000000)" 0.0)))
                (Default|SetContentAlpha (Utilities|Array|Get(acopy) (Variables|Default|GetSlideArray) (Variables|Default|Getindex)) _linearcurve))
              (:Finished
                (for _array_element (Variables|/PresentationPlugin/SlideBP.SlideBP_C|GetTriggers (Utilities|Array|Get(acopy) (Variables|Default|GetSlideArray) (Variables|Default|Getindex)))
                  (Class|ISlideTriggerable|Trigger(Message) _array_element))
                (CallFunction|HandleCurrentSlideAutoContinue))))
          (:Is%20Not%20Valid
            (Development|PrintString (Utilities|String|Append "Slide number " (Utilities|String|ToString(Integer) (Variables|Default|Getindex)) " is missing!"))))))))

(event Custom|GotoPreviousSlide
  (if (not (Variables|/PresentationPlugin/presentationUI.presentationUI_C|GetshowSettings (Variables|Default|GetpresentationUI)))
    (Utilities|Time|ClearandInvalidateTimerbyHandle (Variables|Default|GetautoContinueHandle))
    (Utilities|IsValid (Variables|Default|GetoldSlide)
      (:Is%20Valid
        (Default|SetContentAlpha (Variables|Default|GetoldSlide) 0.0))
      (:Is%20Not%20Valid
        _))
    (Utilities|IsValid (Utilities|Array|Get(acopy) (Variables|Default|GetSlideArray) (Variables|Default|Getindex))
      (:Is%20Valid
        (Variables|Default|SetoldSlide (Utilities|Array|Get(acopy) (Variables|Default|GetSlideArray) (Variables|Default|Getindex))))
      (:Is%20Not%20Valid
        _))
    (Math|Integer|DecrementInt (Variables|Default|Getindex)
      (:%20%20
        (Variables|Default|SetforwardDirection false)
        (if (< (Variables|Default|Getindex) 0)
          (Variables|Default|Setindex (- (Utilities|Array|Length (Variables|Default|GetSlideArray)) 1)))
        (Variables|Default|Setoldtransform (Transformation|GetWorldTransform (Variables|Default|GetCamera)))
        (Utilities|ContinueifSlidesExist)
        (Utilities|IsValid (Utilities|Array|Get(acopy) (Variables|Default|GetSlideArray) (Variables|Default|Getindex))
          (:Is%20Valid
            (Variables|Default|Setnewtransform (Transformation|GetWorldTransform (Variables|/PresentationPlugin/SlideBP.SlideBP_C|GetArrow (Utilities|Array|Get(acopy) (Variables|Default|GetSlideArray) (Variables|Default|Getindex)))))
            (Components|Timeline|SetPlayRate (Variables|Default|GetTransition) (/ 1.0 (Variables|/PresentationPlugin/SlideBP.SlideBP_C|GettransitionDuration (select (Variables|Default|GetforwardDirection) (Utilities|Array|Get(acopy) (Variables|Default|GetSlideArray) (Variables|Default|Getindex)) (Variables|Default|GetoldSlide)))))
            (bind (_direction _smoothcurve _linearcurve) (Timeline|Transition PlayFromStart)
              (:Update
                (Transformation|SetWorldLocationAndRotation (Variables|Default|GetCamera) (Math|Vector|SelectVector (Spline|GetLocationatDistanceAlongSpline (Variables|/PresentationPlugin/SlideBP.SlideBP_C|GetSpline (select (Variables|Default|GetforwardDirection) (Utilities|Array|Get(acopy) (Variables|Default|GetSlideArray) (Variables|Default|Getindex)) (Variables|Default|GetoldSlide))) (* (select (Variables|Default|GetforwardDirection) _smoothcurve (- 1.0 _smoothcurve)) (Spline|GetSplineLength (Variables|/PresentationPlugin/SlideBP.SlideBP_C|GetSpline (select (Variables|Default|GetforwardDirection) (Utilities|Array|Get(acopy) (Variables|Default|GetSlideArray) (Variables|Default|Getindex)) (Variables|Default|GetoldSlide))))) "World") (Math|Vector|Lerp(Vector) (.location (Variables|Default|Getoldtransform)) (.location (Variables|Default|Getnewtransform)) _smoothcurve) (and (Variables|/PresentationPlugin/SlideBP.SlideBP_C|GethasTransitionBeginning (select (Variables|Default|GetforwardDirection) (Utilities|Array|Get(acopy) (Variables|Default|GetSlideArray) (Variables|Default|Getindex)) (Variables|Default|GetoldSlide))) (Variables|/PresentationPlugin/SlideBP.SlideBP_C|GetuseComplexPath (select (Variables|Default|GetforwardDirection) (Utilities|Array|Get(acopy) (Variables|Default|GetSlideArray) (Variables|Default|Getindex)) (Variables|Default|GetoldSlide))))) (Math|Rotator|Lerp(Rotator) (.rotation (Variables|Default|Getoldtransform)) (.rotation (Variables|Default|Getnewtransform)) _smoothcurve true) false false)
                (Utilities|IsValid (Variables|Default|GetoldSlide)
                  (:Is%20Valid
                    (Default|SetContentAlpha (Variables|Default|GetoldSlide) (- 1.0 _linearcurve)))
                  (:Is%20Not%20Valid
                    (Development|PrintString "A Slide is missing!" true true "(R=0.000000,G=0.660000,B=1.000000,A=1.000000)" 0.0)))
                (Default|SetContentAlpha (Utilities|Array|Get(acopy) (Variables|Default|GetSlideArray) (Variables|Default|Getindex)) _linearcurve))
              (:Finished
                (for _array_element (Variables|/PresentationPlugin/SlideBP.SlideBP_C|GetTriggers (Utilities|Array|Get(acopy) (Variables|Default|GetSlideArray) (Variables|Default|Getindex)))
                  (Class|ISlideTriggerable|Trigger(Message) _array_element))
                (CallFunction|HandleCurrentSlideAutoContinue))))
          (:Is%20Not%20Valid
            (Development|PrintString (Utilities|String|Append "Slide number " (Utilities|String|ToString(Integer) (Variables|Default|Getindex)) " is missing!"))))))))

(event Custom|HandleCurrentSlideAutoContinue
  (bind _slidearray (Variables|Default|GetSlideArray))
  (bind _index (Variables|Default|Getindex))
  (bind _output (Utilities|Array|Get(acopy) _slidearray _index))
  (bind _autocontinuetime (Variables|/PresentationPlugin/SlideBP.SlideBP_C|GetautoContinueTime _output))
  (if (!= _autocontinuetime 0.0)
    (bind _returnvalue (Utilities|Time|SetTimerbyFunctionName 0 "GotoNextSlide" _autocontinuetime))
    (Variables|Default|SetautoContinueHandle _returnvalue)))

(event EventBeginPlay
  (Variables|/Script/Engine.PlayerController|SetbShowMouseCursor (Game|GetPlayerController 0) true)
  (bind _returnvalue (UserInterface|CreateWidget "/PresentationPlugin/presentationUI.presentationUI_C"))
  (bind _output_get (Variables|Default|SetpresentationUI _returnvalue))
  (UserInterface|Viewport|AddtoViewport _output_get 0)
  (|EvaluatePlatform)
  (CallFunction|SortSlides (Variables|Default|GetSlideArray))
  (Utilities|ContinueifSlidesExist)
  (Transformation|SetWorldTransform (Variables|Default|GetCamera) (Transformation|GetWorldTransform (Variables|/PresentationPlugin/SlideBP.SlideBP_C|GetArrow (Utilities|Array|Get(acopy) (Variables|Default|GetSlideArray)))) false false)
  (for (_array_element _array_index) (Variables|Default|GetSlideArray)
    (Utilities|IsValid _array_element
      (:Is%20Valid
        (Class|WidgetComponent|SetDrawSize (Variables|/PresentationPlugin/SlideBP.SlideBP_C|GetWidget _array_element) (/ (Viewport|GetViewportSize) 2.0)))
      (:Is%20Not%20Valid
        (Development|PrintString (Utilities|String|Append "Slide number " (Utilities|String|ToString(Integer) _array_index) " is missing!")))))
  (Utilities|FlowControl|Delay 0.0)
  (for (_array_element_2 _array_index_2) (Variables|Default|GetSlideArray)
    (if (!= _array_index_2 0)
      (Utilities|IsValid _array_element_2
        (:Is%20Valid
          (Default|SetContentAlpha _array_element_2 0.0))
        (:Is%20Not%20Valid
          (Development|PrintString (Utilities|String|Append "Slide number " (Utilities|String|ToString(Integer) _array_index_2) " is missing!"))))))
  (CallFunction|HandleCurrentSlideAutoContinue))

(event Input|MouseEvents|LeftMouseButton
  (params (Key :type Key%20Structure :default "AnyKey"))
  (:Pressed
    (CallFunction|GotoNextSlide)))

(event Input|MouseEvents|RightMouseButton
  (params (Key :type Key%20Structure :default "AnyKey"))
  (:Pressed
    (CallFunction|GotoPreviousSlide)))

(event Input|KeyboardEvents|Backspace
  (params (Key :type Key%20Structure :default "AnyKey"))
  (:Pressed
    (CallFunction|GotoPreviousSlide)))

(event Input|KeyboardEvents|Escape
  (params (Key :type Key%20Structure :default "AnyKey"))
  (:Pressed
    (Default|ToggleSettings (Variables|Default|GetpresentationUI))))

(event Input|KeyboardEvents|Left
  (params (Key :type Key%20Structure :default "AnyKey"))
  (:Pressed
    (CallFunction|GotoPreviousSlide)))

(event Input|KeyboardEvents|Right
  (params (Key :type Key%20Structure :default "AnyKey"))
  (:Pressed
    (CallFunction|GotoNextSlide)))

(event Input|KeyboardEvents|Enter
  (params (Key :type Key%20Structure :default "AnyKey"))
  (:Pressed
    (CallFunction|GotoNextSlide)))

(event Input|KeyboardEvents|SpaceBar
  (params (Key :type Key%20Structure :default "AnyKey"))
  (:Pressed
    (CallFunction|GotoNextSlide)))

(event Input|TouchEvents|InputTouch
  (params (Location :type Vector) (FingerIndex :type ETouchIndex%20Enum))
  (bind _returnvalue (Utilities|Enum|Equal(Enum) FingerIndex "Touch1"))
  (bind _istouchdevice (Variables|Default|GetisTouchDevice))
  (bind _returnvalue_2 (and _returnvalue _istouchdevice))
  (:Pressed
    (if _returnvalue_2
      (Variables|Default|Settouchstart (Math|DateTime|Now))))
  (:Released
    (if _returnvalue_2
      (if (<= (Class|KismetMathLibrary|GetTotalMilliseconds (- (Math|DateTime|Now) (Variables|Default|Gettouchstart))) 2.5e+02)
        (if (> (/ (.X (Math|Vector2D|BreakVector2D (Viewport|GetViewportSize))) (.X (Math|Vector|BreakVector Location))) 0.5)
          (CallFunction|GotoNextSlide)
          (else
            (CallFunction|GotoPreviousSlide)))))))

(fn ConstructionScript
  (bind _outactors (Actor|GetAllActorsOfClass "/PresentationPlugin/SlideBP.SlideBP_C"))
  (Variables|Default|SetSlideArray _outactors))

(fn SortSlides
  (params (Array :type Array%20of%20Slide%20BP%20Object%20References))
  (for _array_element Array
    (Utilities|IsValid _array_element
      (:Is%20Valid
        (Utilities|Array|SetArrayElem (LocalVariables|GetSlideArraySort) (Variables|/Script/PresentationRuntimeModule.Slide|GetSlideIndex _array_element) _array_element true))))
  (Variables|Default|SetSlideArray (LocalVariables|GetSlideArraySort)))