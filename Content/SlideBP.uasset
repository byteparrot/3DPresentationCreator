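; SlideBP is a placeable presentation slide actor that shows a templated layout on a widget component in the world.
; UpdateSlide, run on construction and BeginPlay, builds the widget for the chosen style, fills in its data and auto-assigns an unset index.
; It also anchors a hidden transition spline to the previous slide's arrow.
; Index functions swap order with neighboring slides, and Tick scales draw size to the viewport.
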(event EventBeginPlay
  (CallFunction|UpdateSlide))

(event EventTick
  (params (DeltaSeconds :type Float%20%28single-precision%29))
  (CallFunction|SetSlidetoViewportSize))

(fn ConstructionScript
  (CallFunction|UpdateSlide))

(fn GetWidgetfromStyle
  (params (SlideStyle :type SlideStyle%20Enum))
  (switch Utilities|FlowControl|Switch|SwitchonSlideStyle SlideStyle
    (:NewEnumerator0
      (bind _returnvalue (UserInterface|CreateWidget "/PresentationPlugin/Slide_Basic.Slide_Basic_C"))
      (return _returnvalue))
    (:NewEnumerator1
      (bind _returnvalue_2 (UserInterface|CreateWidget "/PresentationPlugin/Slide_Big.Slide_Big_C"))
      (return _returnvalue_2))
    (:NewEnumerator2
      (bind _returnvalue_3 (UserInterface|CreateWidget "/PresentationPlugin/Slide_SmallLeft.Slide_SmallLeft_C"))
      (return _returnvalue_3))
    (:NewEnumerator3
      (bind _returnvalue_4 (UserInterface|CreateWidget "/PresentationPlugin/Slide_SmallRight.Slide_SmallRight_C"))
      (return _returnvalue_4))
    (:NewEnumerator4
      (bind _returnvalue_5 (UserInterface|CreateWidget "/PresentationPlugin/Slide_TwoColumn.Slide_TwoColumn_C"))
      (return _returnvalue_5))
    (:NewEnumerator5
      (bind _returnvalue_6 (UserInterface|CreateWidget "/PresentationPlugin/Slide_OneColumn_TwoColumn.Slide_OneColumn_TwoColumn_C"))
      (return _returnvalue_6))
    (:NewEnumerator7
      (bind _returnvalue_7 (UserInterface|CreateWidget "/PresentationPlugin/Slide_Title1.Slide_Title1_C"))
      (return _returnvalue_7))
    (:NewEnumerator8
      (bind _returnvalue_8 (UserInterface|CreateWidget "/PresentationPlugin/Slide_Title2.Slide_Title2_C"))
      (return _returnvalue_8))
    (:NewEnumerator9
      (bind _returnvalue_9 (UserInterface|CreateWidget "/PresentationPlugin/Slide_SmallUp.Slide_SmallUp_C"))
      (return _returnvalue_9))
    (:NewEnumerator10
      (bind _returnvalue_10 (UserInterface|CreateWidget "/PresentationPlugin/Slide_SmallDown.Slide_SmallDown_C"))
      (return _returnvalue_10))
    (:NewEnumerator11
      (bind _returnvalue_11 (UserInterface|CreateWidget "/PresentationPlugin/Slide_SmallUpLeft.Slide_SmallUpLeft_C"))
      (return _returnvalue_11))
    (:NewEnumerator12
      (bind _returnvalue_12 (UserInterface|CreateWidget "/PresentationPlugin/Slide_SmallUpRight.Slide_SmallUpRight_C"))
      (return _returnvalue_12))
    (:NewEnumerator13
      (bind _returnvalue_13 (UserInterface|CreateWidget "/PresentationPlugin/Slide_SmallDownLeft.Slide_SmallDownLeft_C"))
      (return _returnvalue_13))
    (:NewEnumerator14
      (bind _returnvalue_14 (UserInterface|CreateWidget "/PresentationPlugin/Slide_SmallDownRight.Slide_SmallDownRight_C"))
      (return _returnvalue_14))
    (:NewEnumerator6
      (bind _returnvalue_15 (UserInterface|CreateWidget (Variables|Default|GetCustomTemplate)))
      (return _returnvalue_15))))

(fn UpdateSlide
  ;[1 1 1] Set Slide UMG Design
  (bind _returnvalue (CallFunction|GetWidgetfromStyle (Variables|Default|GetSlideTemplate)))
  (bind _output_get (Variables|Default|SetSlide _returnvalue))
  (Default|SetContent _output_get (Variables|Default|GetData))
  (UserInterface|SetWidget (Variables|Default|GetWidget) _output_get)
  ;[1 1 1] Set Initial Slide Index
  (if (== (Variables|Default|GetSlideIndex) -1)
    (bind _outactors (Actor|GetAllActorsOfClass "SlideBP_C"))
    (Variables|Default|SetSlideIndex (- (Utilities|Array|Length _outactors) 1)))
  (CallFunction|SetSlidetoViewportSize)
  ;[1 1 1] Transition Spline
  (bind _outactors_2 (Actor|GetAllActorsOfClass "SlideBP_C"))
  (bind _array_element (Utilities|Array|ForEachLoopwithBreak _outactors_2 :!label _label)
    (:LoopBody
      (if (== (Variables|/Script/PresentationRuntimeModule.Slide|GetSlideIndex _array_element) (- (Variables|Default|GetSlideIndex) 1))
        (Spline|SetLocationatSplinePoint (Variables|Default|GetSpline) 0 (Transformation|GetWorldLocation (Variables|SlideBP_C|GetArrow _array_element)) "World" true)
        (Variables|Default|SethasTransitionBeginning true)
        (goto _label Break)
        (else
          (Variables|Default|SethasTransitionBeginning false))))
    (:Completed
      (Rendering|SetVisibility (Variables|Default|GetSpline) false false))))

(fn ResetTransitionCurve
  (bind _spline (Variables|Default|GetSpline))
  (bind _returnvalue (Spline|GetNumberOfSplinePoints _spline))
  (if (> _returnvalue 2)
    (for _index (range 1 (- _returnvalue 1))
      (Spline|RemoveSplinePoint (Variables|Default|GetSpline) _index true)))
  (Spline|SetLocationatSplinePoint (Variables|Default|GetSpline) (- (Spline|GetNumberOfSplinePoints (Variables|Default|GetSpline)) 1) (Math|Vector|MakeVector 0.0 0.0 0.0) "Local" true)
  (CallFunction|UpdateSlide))

(fn SetContentAlpha
  (params (Alpha :type Float%20%28single-precision%29))
  (Class|ISlide|SetContentAlpha(Message) (Variables|Default|GetSlide) Alpha))

(fn SetSlidetoViewportSize
  (bind _returnvalue (Viewport|GetViewportSize))
  (bind _widget (Variables|Default|GetWidget))
  ;[1 1 1] Adapt Size To Resolution
  (bind _returnvalue_2 (Class|Slide|GetViewportSize))
  (Class|WidgetComponent|SetDrawSize _widget (/ (select (Math|Vector|Equal(Vector) _returnvalue "(X=1.000000,Y=1.000000)" 2.0) _returnvalue_2 _returnvalue) (Math|Float|MapRangeUnclamped (.X (Math|Vector2D|BreakVector2D (select (Math|Vector|Equal(Vector) _returnvalue "(X=1.000000,Y=1.000000)" 2.0) _returnvalue_2 _returnvalue))) 7e+02 1.92e+03 0.71 1.93)))
  (Class|WidgetComponent|RequestRedraw _widget)
  (if (Math|Vector|NotEqual(Vector) (select (Math|Vector|Equal(Vector) _returnvalue "(X=1.000000,Y=1.000000)" 2.0) _returnvalue_2 _returnvalue) (Variables|Default|GetlastDrawSize) 0.0001)
    _
    (else
      _))
  (Variables|Default|SetlastDrawSize (select (Math|Vector|Equal(Vector) _returnvalue "(X=1.000000,Y=1.000000)" 2.0) _returnvalue_2 _returnvalue)))

(fn IncrementSlideIndex
  (bind _returnvalue (Class|Slide|GetLastSlideNumber))
  (if (== _returnvalue (Variables|Default|GetSlideIndex))
    (Development|PrintString "Current Slide is Already Last Slide! Inkrementing Anyways")
    (Math|Integer|IncrementInt (Variables|Default|GetSlideIndex))
    (else
      (bind _outactors (Actor|GetAllActorsOfClass "SlideBP_C"))
      (bind _array_element (Utilities|Array|ForEachLoopwithBreak _outactors :!label _label)
        (:LoopBody
          (if (== (Variables|/Script/PresentationRuntimeModule.Slide|GetSlideIndex _array_element) (+ (Variables|Default|GetSlideIndex) 1))
            (LocalVariables|SetConflictSolved true)
            (Variables|/Script/PresentationRuntimeModule.Slide|SetSlideIndex _array_element (Variables|Default|GetSlideIndex))
            (Math|Integer|IncrementInt (Variables|Default|GetSlideIndex)
              (:%20%20
                (CallFunction|UpdateSlide _array_element)
                (CallFunction|UpdateSlide)
                (goto _label Break)))))
        (:Completed
          (if (not (LocalVariables|GetConflictSolved))
            (Development|PrintString "Next Slide not found")
            (Math|Integer|IncrementInt (Variables|Default|GetSlideIndex))))))))

(fn DecrementSlideIndex
  (if (== 0 (Variables|Default|GetSlideIndex))
    (Development|PrintString "Current Slide is Already First!")
    (else
      (bind _outactors (Actor|GetAllActorsOfClass "SlideBP_C"))
      (bind _array_element (Utilities|Array|ForEachLoopwithBreak _outactors :!label _label)
        (:LoopBody
          (if (== (Variables|/Script/PresentationRuntimeModule.Slide|GetSlideIndex _array_element) (- (Variables|Default|GetSlideIndex) 1))
            (LocalVariables|SetConflictSolved true)
            (Variables|/Script/PresentationRuntimeModule.Slide|SetSlideIndex _array_element (Variables|Default|GetSlideIndex))
            (Math|Integer|DecrementInt (Variables|Default|GetSlideIndex)
              (:%20%20
                (CallFunction|UpdateSlide _array_element)
                (CallFunction|UpdateSlide)
                (goto _label Break)))))
        (:Completed
          (if (not (LocalVariables|GetConflictSolved))
            (Development|PrintString "Previous Slide not found")
            (Math|Integer|DecrementInt (Variables|Default|GetSlideIndex))))))))